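; BP_MyPlayerController is a player controller Blueprint that animates the pause menu when it is shown and removed.
; It extends the parent's DisplayPauseMenu and RemovePauseMenu events, casting PauseMenu to WBP_PauseMenu to play its PauseMenuAnimation forward on display and in reverse on removal.
; On removal, a short fixed delay follows the reverse animation before the widget is set to Hidden.
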(event EventDisplayPauseMenu
  (|CallParentFunction)
  (bind _aswbp_pause_menu (Utilities|Casting|CastToWBP_PauseMenu (Variables|Default|GetPauseMenu)))
  (UserInterface|Animation|PlayAnimation _aswbp_pause_menu (Variables|/Game/Blueprints/GameplayMechanics/Widget/WBP_PauseMenu.WBP_PauseMenu_C|GetPauseMenuAnimation _aswbp_pause_menu) 0.0 1 "Forward" 1.0))

(event EventRemovePauseMenu
  (|CallParentFunction)
  (bind _aswbp_pause_menu (Utilities|Casting|CastToWBP_PauseMenu (Variables|Default|GetPauseMenu)))
  (UserInterface|Animation|PlayAnimation _aswbp_pause_menu (Variables|/Game/Blueprints/GameplayMechanics/Widget/WBP_PauseMenu.WBP_PauseMenu_C|GetPauseMenuAnimation _aswbp_pause_menu) 0.0 1 "Reverse" 1.0)
  (Utilities|FlowControl|Delay 0.25)
  (Widget|SetVisibility (Variables|Default|GetPauseMenu) "Hidden"))

(fn ConstructionScript)